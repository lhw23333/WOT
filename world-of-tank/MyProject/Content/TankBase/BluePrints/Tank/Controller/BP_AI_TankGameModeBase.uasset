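; Game mode for a Red versus Blue tank match that decides the winner and ends the game.
; It records players on login, and setting a player's info also binds every controller's pawn-death event.
; Each death triggers a scan of living pawns by group to find whether one side is eliminated.
; Game over shows the result through the player controllers, then opens the start map after a delay.
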(event `self.K2_PostLogin`
  (params (NewPlayer :type "PlayerController Object Reference"))
  (`KismetArrayLibrary.Array_AddUnique` (`self.PlayerList`) NewPlayer))

(event `EVE_SetPlayerInfo`
  (params (PlayerInfo :type "/Game/TankBase/UI/Str_Player_info Structure") (PlayerController :type "/Game/TankBase/BluePrints/Tank/Controller/BP_TankPlayerController Object Reference"))
  ;[1 1 1] 修改PlayerInfo信息
  (set `/Game/TankBase/BluePrints/Tank/Controller/BP_TankPlayerController.PlayerInfo` PlayerInfo PlayerController)
  (for _array_element (`self.PlayerList`)
    (bind _asbp_tank_player_controller (cast `/Game/TankBase/BluePrints/Tank/Controller/BP_TankPlayerController` _array_element))
    (add `TankPlayerController.OnPawnDeath` _asbp_tank_player_controller (delegate `OnPawnDeath_Event`))))

(event `OnPawnDeath_Event`
  ;[1 1 1] 修改PlayerInfo信息
  (set `self.RedWin` true)
  (set `self.BlueWin` true)
  (for _array_element (`self.PlayerList`)
    (bind _asbp_tank_player_controller (cast `/Game/TankBase/BluePrints/Tank/Controller/BP_TankPlayerController` _array_element))
    (if (`TankPlayerController.bPawnIsLive` _asbp_tank_player_controller)
      (switch `int` (`.Group_10_6B49C83B4E92B04C761EEBAC208B29BE` (break `/Game/TankBase/UI/Str_Player_info` (`/Game/TankBase/BluePrints/Tank/Controller/BP_TankPlayerController.PlayerInfo` _asbp_tank_player_controller)))
        (:`0`
          (set `self.RedWin` false))
        (:`1`
          (set `self.BlueWin` false)))))
  (if (== (`self.RedWin`) true)
    (`self.EVE_GameOver` "Red Win")
    (elif (== (`self.BlueWin`) true)
      (`self.EVE_GameOver` "Blue Win"))))

(event `EVE_GameOver`
  (params (GameResult :type Text))
  (for _array_element (`self.PlayerList`)
    (bind _asbp_tank_player_controller (cast `/Game/TankBase/BluePrints/Tank/Controller/BP_TankPlayerController` _array_element))
    (`/Game/TankBase/BluePrints/Tank/Controller/BP_TankPlayerController.EVE_ShowGameResult` _asbp_tank_player_controller GameResult)
    (`KismetSystemLibrary.Delay` 5.0)
    (`GameplayStatics.OpenLevel` "Map_Start")))

(fn `UserConstructionScript`)