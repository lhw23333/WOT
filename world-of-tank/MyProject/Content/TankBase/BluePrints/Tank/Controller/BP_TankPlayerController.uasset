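; Player controller for the tank game that manages the local UI and passes player info into the match.
; BeginPlay creates the main and inventory widgets, then sends PlayerInfo from the GameIn_Main game instance to BP_TankGameModeBase.
; On possession, after a short delay, it copies the player's Group to the tank and binds its death event.
; Death and match result events clear all widgets to show the YouDead or GameOver screen.
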(event `self.ReceiveBeginPlay`
  (bind _returnvalue (`|CreateWidget` "/Game/TankBase/BluePrints/TankUI/MainUI.MainUI_C" self))
  (`UserWidget.AddToViewport` _returnvalue 0)
  (bind _returnvalue_2 (`self.GetControlledTankVehicle`))
  (bind _returnvalue_3 (`|CreateWidget` "/Game/InventorySystems/UI/InventoryUI.InventoryUI_C" self))
  (set `/Game/InventorySystems/UI/InventoryUI.Tank` _returnvalue_2 _returnvalue_3)
  (set `self.Inventory` _returnvalue_3)
  (`UserWidget.AddToViewport` _returnvalue_3 0)
  (`self.EVE_Init`))

(event `self.ReceivePossess`
  (params (PossessedPawn :type "Pawn Object Reference"))
  ;[1 1 1] 初始化坦克阵营
  (`KismetSystemLibrary.Delay` 1.0)
  (bind _asbp_tank_vehicle (cast `/Game/VigilanteContent/Vehicles/West_Tank_M1A1Abrams/BP_TankVehicle` PossessedPawn))
  (set `/Game/VigilanteContent/Vehicles/West_Tank_M1A1Abrams/BP_TankVehicle.Group` (`.Group_10_6B49C83B4E92B04C761EEBAC208B29BE` (break `/Game/TankBase/UI/Str_Player_info` (`self.PlayerInfo`))) _asbp_tank_vehicle)
  (add `TankVehicle.OnDeath` _asbp_tank_vehicle (delegate `EVE_OnDeath`)))

(event `EVE_OnDeath`
  ;[1 1 1] 初始化坦克阵营
  (`WidgetLayoutLibrary.RemoveAllWidgets`)
  (bind _returnvalue (`|CreateWidget` "/Game/TankBase/UI/YouDead.YouDead_C" self))
  (`UserWidget.AddToViewport` _returnvalue 0)
  (set `PlayerController.bShowMouseCursor` true (`GameplayStatics.GetPlayerController` 0)))

(event `EVE_Init`
  ;[1 1 1] 初始化PlayerInfo信息
  (bind _asgame_in_main (cast `/Game/TankBase/UI/GameIn_Main` (`GameplayStatics.GetGameInstance`)))
  (`self.EVE_SetPlayerInfo` (`/Game/TankBase/UI/GameIn_Main.PlayerInfo` _asgame_in_main)))

(event `EVE_SetPlayerInfo`
  (params (PlayerInfo :type "/Game/TankBase/UI/Str_Player_info Structure"))
  ;[1 1 1] 初始化PlayerInfo信息
  (bind _asbp_tank_game_mode_base (cast `/Game/TankBase/BluePrints/Tank/Controller/BP_TankGameModeBase` (`GameplayStatics.GetGameMode`)))
  (`/Game/TankBase/BluePrints/Tank/Controller/BP_TankGameModeBase.EVE_SetPlayerInfo` _asbp_tank_game_mode_base PlayerInfo self))

(event `EVE_ShowGameResult`
  (params (GameResult :type Text))
  (`KismetSystemLibrary.Delay` 0.2)
  (`WidgetLayoutLibrary.RemoveAllWidgets`)
  (bind _returnvalue (`|CreateWidget` "/Game/TankBase/UI/GameOver.GameOver_C"))
  (`UserWidget.AddToViewport` _returnvalue 0)
  (set `/Game/TankBase/UI/GameOver.WhoWin` GameResult _returnvalue))

(fn `OnRep_PlayerInfo`)

(fn `UserConstructionScript`)