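; AI controller for enemy tanks that provides spline patrol and player-facing attack driving behaviors.
; After a short startup delay it sets the tank's group, runs its behavior tree and clears the attack-mode blackboard flag.
; Patrol drives at half throttle toward a look-ahead point on the first path's spline.
; Attack cuts throttle and steers toward the player tank with a debug line, both mapping yaw error to steering.
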(event `self.ReceiveBeginPlay`
  (`KismetSystemLibrary.Delay` 0.2)
  (bind _returnvalue (`self.GetControlledTank`))
  (bind _asbp_tank_vehicle (cast `/Game/VigilanteContent/Vehicles/West_Tank_M1A1Abrams/BP_TankVehicle` _returnvalue))
  (set `/Game/VigilanteContent/Vehicles/West_Tank_M1A1Abrams/BP_TankVehicle.Group` 1 _asbp_tank_vehicle)
  (`self.RunBehaviorTree` "/Game/VigilanteContent/Vehicles/AI/AI_BehaviorTree.AI_BehaviorTree")
  (bind _blackboardcomponent (`self.UseBlackboard` "/Game/VigilanteContent/Vehicles/AI/AI_BlackboardData.AI_BlackboardData"))
  (`BlackboardComponent.SetValueAsBool` _blackboardcomponent "IsAttackMode" false))

(event `EVE_Attack`
  (`WheeledVehicleMovementComponent.SetThrottleInput` (`WheeledVehicle.VehicleMovement` (cast `TankVehicle` (`self.K2_GetPawn`) :!pure true)) 0.0)
  (bind _returnvalue (`self.GetPlayerTank`))
  (bind _steeing (`self.MoveToPlayer` _returnvalue))
  (`WheeledVehicleMovementComponent.SetSteeringInput` (`WheeledVehicle.VehicleMovement` (cast `TankVehicle` (`self.K2_GetPawn`) :!pure true)) _steeing))

(event `EVE_Patrol`
  ;[1 1 1] AI巡逻
  (`WheeledVehicleMovementComponent.SetThrottleInput` (`WheeledVehicle.VehicleMovement` (cast `TankVehicle` (`self.K2_GetPawn`) :!pure true)) 0.5)
  (bind _outactors (`GameplayStatics.GetAllActorsOfClass` "/Game/VigilanteContent/Vehicles/AI/Path.Path_C"))
  (bind _steering (`self.Get Path` _outactors))
  (`WheeledVehicleMovementComponent.SetSteeringInput` (`WheeledVehicle.VehicleMovement` (cast `TankVehicle` (`self.K2_GetPawn`) :!pure true)) _steering))

(fn `Get Path`
  (params (Path :type "Array of /Game/VigilanteContent/Vehicles/AI/Path Object Reference"))
  (returns (Steering :type "Float (double-precision)"))
  (bind _returnvalue (`self.K2_GetActorLocation` (`self.K2_GetPawn`)))
  (bind _spline (`/Game/VigilanteContent/Vehicles/AI/Path.Spline` (`|GetArrayItem` Path)))
  (bind (_returnvalue_roll _returnvalue_pitch _returnvalue_yaw) (`KismetMathLibrary.BreakRotator` (`KismetMathLibrary.NormalizedDeltaRotator` (`KismetMathLibrary.FindLookAtRotation` _returnvalue (`SplineComponent.FindLocationClosestToWorldLocation` _spline (+ (* (`KismetMathLibrary.Normal` (`SplineComponent.FindTangentClosestToWorldLocation` _spline _returnvalue "World")) 500.0) _returnvalue) "World")) (`self.K2_GetActorRotation` (`self.K2_GetPawn`)))))
  (return (`KismetMathLibrary.MapRangeClamped` _returnvalue_yaw -90.0 90.0 -1.0 1.0)))

(fn `MoveToPlayer`
  (params (TargetActor :type "Actor Object Reference"))
  (returns (Steeing :type "Float (double-precision)"))
  (bind _returnvalue (`self.K2_GetActorLocation` TargetActor))
  (bind _returnvalue_2 (`self.K2_GetActorLocation` (`self.K2_GetPawn`)))
  (bind (_returnvalue_roll _returnvalue_pitch _returnvalue_yaw) (`KismetMathLibrary.BreakRotator` (`KismetMathLibrary.NormalizedDeltaRotator` (`KismetMathLibrary.FindLookAtRotation` _returnvalue_2 _returnvalue) (`self.K2_GetActorRotation` (`self.K2_GetPawn`)))))
  (`KismetSystemLibrary.DrawDebugLine` _returnvalue_2 _returnvalue (struct :`A` 1.0) 0.1 20.0)
  (return (`KismetMathLibrary.MapRangeClamped` _returnvalue_yaw -90.0 90.0 -1.0 1.0)))

(fn `UserConstructionScript`)