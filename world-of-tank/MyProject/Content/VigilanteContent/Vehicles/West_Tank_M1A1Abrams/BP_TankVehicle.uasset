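; BP_TankVehicle is a drivable M1A1 Abrams tank Blueprint with player camera and movement controls.
; Look axes yaw the SpringArm freely and adjust its pitch within a clamped range.
; Move axes feed the VehicleMovement component, passing steering through directly while throttle is effectively doubled and clamped, reaching full power at half input.
; The graph holds only input handling, with no turret, weapon or construction logic.
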(event `InputAxis|LookH`
  (params (AxisValue :type "Float (single-precision)"))
  ;[1 1 1] 视角控制
  (`SceneComponent.K2_AddRelativeRotation` (`self.SpringArm`) (`KismetMathLibrary.MakeRotator` 0.0 0.0 AxisValue) false false))

(event `InputAxis|LookV`
  (params (AxisValue :type "Float (single-precision)"))
  (bind (_relativerotation_roll _relativerotation_pitch _relativerotation_yaw) (`KismetMathLibrary.BreakRotator` (`SceneComponent.RelativeRotation` (`self.SpringArm`))))
  ;[1 1 1] 视角控制
  (`SceneComponent.K2_SetRelativeRotation` (`self.SpringArm`) (`KismetMathLibrary.MakeRotator` _relativerotation_roll (`KismetMathLibrary.FClamp` (+ AxisValue _relativerotation_pitch) -80.0 20.0) _relativerotation_yaw) false false))

(event `self.ReceiveBeginPlay`)

(event `InputAxis|MoveForward`
  (params (AxisValue :type "Float (single-precision)"))
  (bind _returnvalue (`KismetMathLibrary.Abs` (`self.Axis Value`)))
  ;[1 1 1] 移动载具
  (`WheeledVehicleMovementComponent.SetThrottleInput` (`self.VehicleMovement`) (`KismetMathLibrary.FClamp` (+ AxisValue (`KismetMathLibrary.SelectFloat` (* -1.0 _returnvalue) _returnvalue (< AxisValue 0.0))) -1.0)))

(event `InputAxis|MoveRight`
  (params (AxisValue :type "Float (single-precision)"))
  ;[1 1 1] 移动载具
  (bind _output_get (set `self.Axis Value` AxisValue))
  (`WheeledVehicleMovementComponent.SetSteeringInput` (`self.VehicleMovement`) _output_get))

(fn `UserConstructionScript`)